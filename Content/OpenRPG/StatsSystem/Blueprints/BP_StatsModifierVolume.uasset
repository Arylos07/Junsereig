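; Trigger volume that applies a buff and effects to an overlapping master character through its player controller's stats handler component.
; The construction script loads its DT_Volumes row by ID and builds the box, plus optional mesh and particles.
; On exit, only While Overlapping mode removes the buff and effects.
; DoOnce gates on enter and exit reset unless the volume is single-use, with the exit reset limited to that mode.
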(event Collision|EventActorBeginOverlap
  (params (OtherActor :type Actor%20Object%20Reference))
  (bind _volumemodifierinfo (Variables|Default|GetVolumeModifierInfo))
  (bind (_buff _effects _useonlyonce_) (Utilities|Struct|Breaks_VolumeModifier _volumemodifierinfo))
  (bind _asbp_master_character (Utilities|Casting|CastToBP_MasterCharacter OtherActor))
  (Variables|Default|SetStatsComponent (Variables|/Game/OpenRPG/Shared/Blueprints/BP_CustomPlayerController.BP_CustomPlayerController_C|GetBPC_StatsHandler (Variables|/Game/OpenRPG/Shared/Blueprints/BP_MasterCharacter.BP_MasterCharacter_C|GetBP_PlayerController _asbp_master_character)))
  (Utilities|FlowControl|DoOnce false :!label _label
    (:Completed
      (Default|ApplyBuff (Variables|Default|GetStatsComponent) _buff)
      (for _array_element _effects
        (Default|ApplyEffect (Variables|Default|GetStatsComponent) _array_element))
      (if (not _useonlyonce_)
        (goto _label Reset)))))

(event Collision|EventActorEndOverlap
  (params (OtherActor :type Actor%20Object%20Reference))
  (bind _volumemodifierinfo (Variables|Default|GetVolumeModifierInfo))
  (bind (_buff _effects _useonlyonce_) (Utilities|Struct|Breaks_VolumeModifier _volumemodifierinfo))
  (bind _asbp_master_character (Utilities|Casting|CastToBP_MasterCharacter OtherActor))
  (Variables|Default|SetStatsComponent (Variables|/Game/OpenRPG/Shared/Blueprints/BP_CustomPlayerController.BP_CustomPlayerController_C|GetBPC_StatsHandler (Variables|/Game/OpenRPG/Shared/Blueprints/BP_MasterCharacter.BP_MasterCharacter_C|GetBP_PlayerController _asbp_master_character)))
  (Utilities|FlowControl|DoOnce false :!label _label
    (:Completed
      (switch Utilities|FlowControl|Switch|Switchone_VolumeModifierMode (Utilities|Struct|Breaks_VolumeModifier (Variables|Default|GetVolumeModifierInfo))
        (:NewEnumerator1
          (Default|RemoveBuff (Variables|Default|GetStatsComponent) (Utilities|Struct|Breaks_Buff _buff))
          (for _array_element _effects
            (Default|RemoveEffect (Variables|Default|GetStatsComponent) (Utilities|Struct|Breaks_Effect _array_element)))
          (if (not _useonlyonce_)
            (goto _label Reset)))))))

(fn ConstructionScript
  (bind _returnvalue (Utilities|GetDataTableRow "/Game/OpenRPG/StatsSystem/DataTables/DT_Volumes.DT_Volumes" (Utilities|String|StringToName (Utilities|String|ToString(Integer) (Variables|Default|GetID))))
    (:then
      (Variables|Default|SetVolumeModifierInfo _returnvalue)
      (bind _returnvalue_2 (AddComponent|AddBoxComponent false))
      (Components|Box|SetBoxExtent _returnvalue_2 (Math|Vector|MakeVector (Utilities|Struct|Breaks_VolumeModifier (Variables|Default|GetVolumeModifierInfo)) (Utilities|Struct|Breaks_VolumeModifier (Variables|Default|GetVolumeModifierInfo)) (Utilities|Struct|Breaks_VolumeModifier (Variables|Default|GetVolumeModifierInfo))) false)
      (Utilities|IsValid (.Mesh (Utilities|Struct|Breaks_VolumeModifier (Variables|Default|GetVolumeModifierInfo)))
        (:Is%20Valid
          (bind _returnvalue_3 (AddComponent|AddStaticMeshComponent false (.MeshTransform (Utilities|Struct|Breaks_VolumeModifier (Variables|Default|GetVolumeModifierInfo)))))
          (Components|StaticMesh|SetStaticMesh _returnvalue_3 (.Mesh (Utilities|Struct|Breaks_VolumeModifier (Variables|Default|GetVolumeModifierInfo)))))
        (:Is%20Not%20Valid
          _))
      (Utilities|IsValid (.ParticleEffect (Utilities|Struct|Breaks_VolumeModifier (Variables|Default|GetVolumeModifierInfo)))
        (:Is%20Valid
          (bind _returnvalue_4 (AddComponent|AddParticleSystemComponent false (.ParticleTransform (Utilities|Struct|Breaks_VolumeModifier (Variables|Default|GetVolumeModifierInfo)))))
          (Effects|Components|ParticleSystem|SetTemplate _returnvalue_4 (.ParticleEffect (Utilities|Struct|Breaks_VolumeModifier (Variables|Default|GetVolumeModifierInfo)))))))))