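; Master quest actor that tracks one quest's active and completed sub-goals, description, hunt counts and state.
; Completing or failing a sub-goal updates the quest widget and journal, then adds follow-up goals on success or ends the quest through QuestManager.
; Goals are added recursively, auto-completing those whose target the player already obtained.
; OnGoalCompleted and OnGoalFailed are empty event hooks; cancelling removes widgets and notifies QuestManager.
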(event Custom|OnGoalFailed
  (params (GoalIndex :type Integer)))

(event Custom|OnQuestCancelled
  (CallFunction|RemoveWidgets)
  (Default|CancelQuest (Variables|Donottouch!|GetQuestManager) self))

(event Custom|OnGoalCompleted
  (params (GoalIndex :type Integer)))

(event EventBeginPlay)

(event Collision|EventActorBeginOverlap
  (params (OtherActor :type Actor%20Object%20Reference)))

(event EventTick
  (params (DeltaSeconds :type Float%20%28single-precision%29)))

(fn ConstructionScript)

(fn UpdateSubGoals
  (Utilities|Array|Clear (Variables|Donottouch!|GetCurrentGoals))
  (for _array_element (Variables|Donottouch!|GetCurrentGoalIndices)
    (Utilities|Array|Add (Variables|Donottouch!|GetCurrentGoals) (Utilities|Array|Get(acopy) (.SubGoals (Utilities|Struct|Breaks_QuestInfo (Variables|QuestInformation|GetQuestInfo))) _array_element)))
  (return))

(fn SetupStartingGoals
  (Utilities|Array|Clear (Variables|Donottouch!|GetCurrentGoalIndices))
  (Variables|Donottouch!|SetCurrentDescription (.Description (Utilities|Struct|Breaks_QuestInfo (Variables|QuestInformation|GetQuestInfo))))
  (for _array_element (Variables|QuestInformation|GetStartingSubGoalIndices)
    (CallFunction|AddGoalforIndex _array_element))
  (Utilities|Array|Resize (Variables|Donottouch!|GetCurrentHuntedAmounts) (Utilities|Array|Length (Variables|Donottouch!|GetCurrentGoalIndices)))
  (CallFunction|UpdateSubGoals)
  (return))

(fn GotoNextSubGoal
  (bind _currentgoalindices (Variables|Donottouch!|GetCurrentGoalIndices))
  (bind _currentgoalindices_2 (Variables|Donottouch!|GetCurrentGoalIndices))
  (bind _maxvalue (Math|Integer|MaxOfIntArray _currentgoalindices))
  (bind _returnvalue (+ _maxvalue 1))
  (if (<= _returnvalue (Utilities|Array|LastIndex (.SubGoals (Utilities|Struct|Breaks_QuestInfo (Variables|QuestInformation|GetQuestInfo)))))
    (LocalVariables|SetNextIndex _returnvalue)
    (Utilities|Array|Clear _currentgoalindices_2)
    (Utilities|Array|Add _currentgoalindices_2 (LocalVariables|GetNextIndex))
    (CallFunction|UpdateSubGoals)
    (return true)
    (else
      (return false))))

(fn CompleteSubGoal
  (params (SubGoalIndex :type Integer) (Fail? :type Boolean))
  (bind _currentgoalindices (Variables|Donottouch!|GetCurrentGoalIndices))
  (bind _questwidget (Variables|Donottouch!|GetQuestWidget))
  (bind _questwidget_2 (Variables|Donottouch!|GetQuestWidget))
  (bind _subgoalwidgets (Variables|/Game/QuestSystem/Widgets/QuestWidget.QuestWidget_C|GetSubGoalWidgets _questwidget))
  (LocalVariables|SetlocalFail? Fail?)
  (LocalVariables|SetlocalGoalIndex SubGoalIndex)
  (if (Utilities|Array|ContainsItem (Variables|Donottouch!|GetCurrentGoalIndices) (LocalVariables|GetlocalGoalIndex))
    (bind _output_get (LocalVariables|SetlocalCompletedGoal (Utilities|Array|Get(acopy) (.SubGoals (Utilities|Struct|Breaks_QuestInfo (Variables|QuestInformation|GetQuestInfo))) (LocalVariables|GetlocalGoalIndex))))
    (Utilities|Array|Add (Variables|Donottouch!|GetCompletedSubGoals) (Utilities|Struct|Makes_CompletedGoal (LocalVariables|GetlocalGoalIndex) _output_get (not (LocalVariables|GetlocalFail?))))
    (if (and (.UpdateQuestDescription? (Utilities|Struct|BreakGoalInfo (LocalVariables|GetlocalCompletedGoal))) (not (LocalVariables|GetlocalFail?)))
      (Variables|Donottouch!|SetCurrentDescription (Utilities|Text|FormatText "{Current}{Next}" (Variables|Donottouch!|GetCurrentDescription) (.UpdatedDescription (Utilities|Struct|BreakGoalInfo (LocalVariables|GetlocalCompletedGoal)))))
      (if (CallFunction|SelectedinJournal?)
        (Default|UpdateDescription (Variables|/Game/QuestSystem/Widgets/MainWidget.MainWidget_C|GetJournal (Variables|/Game/QuestSystem/Blueprints/Actors/Bp_QuestManager.Bp_QuestManager_C|GetMainWidget (Variables|Donottouch!|GetQuestManager))))))
    (Utilities|Array|RemoveItem (Variables|Donottouch!|GetCurrentGoals) (LocalVariables|GetlocalCompletedGoal))
    (LocalVariables|SetlocalWidgetIndex (Utilities|Array|FindItem _currentgoalindices (LocalVariables|GetlocalGoalIndex)))
    (Utilities|Array|RemoveIndex (Variables|Donottouch!|GetCurrentHuntedAmounts) (Utilities|Array|FindItem _currentgoalindices (LocalVariables|GetlocalGoalIndex)))
    (Utilities|Array|RemoveItem _currentgoalindices (LocalVariables|GetlocalGoalIndex))
    (Widget|RemovefromParent (Utilities|Array|Get(acopy) _subgoalwidgets (LocalVariables|GetlocalWidgetIndex)))
    (Utilities|Array|RemoveIndex _subgoalwidgets (LocalVariables|GetlocalWidgetIndex))
    (if (LocalVariables|GetlocalFail?)
      (CallFunction|OnGoalFailed (LocalVariables|GetlocalGoalIndex))
      (if (.FailMeansQuestFail? (Utilities|Struct|BreakGoalInfo (LocalVariables|GetlocalCompletedGoal)))
        _
        (else
          (if (CallFunction|SelectedinJournal?) :!label _label
            (Default|GenerateSubGoals (Variables|/Game/QuestSystem/Widgets/MainWidget.MainWidget_C|GetJournal (Variables|/Game/QuestSystem/Blueprints/Actors/Bp_QuestManager.Bp_QuestManager_C|GetMainWidget (Variables|Donottouch!|GetQuestManager)))))
          (if (and (== (LocalVariables|GetlocalGoalIndex) (Variables|Donottouch!|GetSelectedSubGoalIndex)) (== (Variables|/Game/QuestSystem/Blueprints/Actors/Bp_QuestManager.Bp_QuestManager_C|GetCurrentQuest (Variables|Donottouch!|GetQuestManager)) self))
            (Default|SelectSubGoal _questwidget_2 (Utilities|Array|Get(acopy) (Variables|/Game/QuestSystem/Widgets/QuestWidget.QuestWidget_C|GetSubGoalWidgets _questwidget_2)) false))
          (return true)))
      (else
        (CallFunction|OnGoalCompleted (LocalVariables|GetlocalGoalIndex))
        (if (.CompletesQuest? (Utilities|Struct|BreakGoalInfo (LocalVariables|GetlocalCompletedGoal)))
          _
          (else
            (for _array_element (.FollowingSubGoalIndices (Utilities|Struct|BreakGoalInfo (LocalVariables|GetlocalCompletedGoal)))
              (CallFunction|AddGoalforIndex _array_element))
            (goto _label)))))
    (for _array_element_2 (Variables|Donottouch!|GetCurrentGoalIndices)
      (Utilities|Array|Add (Variables|Donottouch!|GetCompletedSubGoals) (Utilities|Struct|Makes_CompletedGoal _array_element_2 (CallFunction|GoalatIndex _array_element_2) false)))
    (Utilities|Array|Clear (Variables|Donottouch!|GetCurrentGoalIndices))
    (Utilities|Array|Clear (Variables|Donottouch!|GetCurrentHuntedAmounts))
    (Utilities|Array|Clear (Variables|Donottouch!|GetCurrentGoals))
    (Variables|Donottouch!|SetCurrentState (select (LocalVariables|GetlocalFail?) "NewEnumerator2" "NewEnumerator1"))
    (CallFunction|RemoveWidgets)
    (Default|EndQuest (Variables|Donottouch!|GetQuestManager) self)
    (return true)
    (else
      (return false))))

(fn SelectedinJournal?
  (bind _questmanager (Variables|Donottouch!|GetQuestManager))
  (bind _mainwidget (Variables|/Game/QuestSystem/Blueprints/Actors/Bp_QuestManager.Bp_QuestManager_C|GetMainWidget _questmanager))
  (bind _journal (Variables|/Game/QuestSystem/Widgets/MainWidget.MainWidget_C|GetJournal _mainwidget))
  (bind _selectedquest (Variables|/Game/QuestSystem/Widgets/QuestJournal.QuestJournal_C|GetSelectedQuest _journal))
  (return (and (Utilities|IsValid _selectedquest) (== _selectedquest self))))

(fn GoalatIndex
  (params (Index :type Integer))
  (return (Utilities|Array|Get(acopy) (.SubGoals (Utilities|Struct|Breaks_QuestInfo (Variables|QuestInformation|GetQuestInfo))) Index)))

(fn GoalAlreadyFound?
  (params (GoalIndex :type Integer))
  (bind _goal (CallFunction|GoalatIndex GoalIndex))
  (bind (_type _customgoal_ _goaltext _additionalname _amounttohunt _goalclass) (Utilities|Struct|BreakGoalInfo _goal))
  (if (Utilities|Enum|Equal(Enum) _type "NewEnumerator2")
    (bind _array_element (Utilities|Array|ForEachLoopwithBreak (Variables|/Game/QuestSystem/Blueprints/Characters/ThirdPersonCharacter.ThirdPersonCharacter_C|GetObtainedObjects (Variables|/Game/QuestSystem/Blueprints/Actors/Bp_QuestManager.Bp_QuestManager_C|GetThirdPersonChar (Variables|Donottouch!|GetQuestManager))) :!label _label)
      (:LoopBody
        (if (== _array_element _goalclass)
          (LocalVariables|SetlocalBool true)
          (goto _label Break)))
      (:Completed
        (return (LocalVariables|GetlocalBool))))
    (else
      (return false))))

(fn AddGoalforIndex
  (params (Index :type Integer))
  (bind _questwidget (Variables|Donottouch!|GetQuestWidget))
  (bind _output_get (LocalVariables|SetlocalIndex Index))
  (if (CallFunction|GoalAlreadyFound? _output_get)
    (Utilities|Array|Add (Variables|Donottouch!|GetCompletedSubGoals) (Utilities|Struct|Makes_CompletedGoal (LocalVariables|GetlocalIndex) (CallFunction|GoalatIndex (LocalVariables|GetlocalIndex)) true))
    (CallFunction|OnGoalCompleted (LocalVariables|GetlocalIndex))
    (if (.UpdateQuestDescription? (Utilities|Struct|BreakGoalInfo (CallFunction|GoalatIndex (LocalVariables|GetlocalIndex))))
      (Variables|Donottouch!|SetCurrentDescription (Utilities|Text|FormatText "{Current}{Next}" (Variables|Donottouch!|GetCurrentDescription) (.UpdatedDescription (Utilities|Struct|BreakGoalInfo (CallFunction|GoalatIndex (LocalVariables|GetlocalIndex))))))
      (if (CallFunction|SelectedinJournal?)
        (Default|UpdateDescription (Variables|/Game/QuestSystem/Widgets/MainWidget.MainWidget_C|GetJournal (Variables|/Game/QuestSystem/Blueprints/Actors/Bp_QuestManager.Bp_QuestManager_C|GetMainWidget (Variables|Donottouch!|GetQuestManager))))))
    (for _array_element (.FollowingSubGoalIndices (Utilities|Struct|BreakGoalInfo (CallFunction|GoalatIndex (LocalVariables|GetlocalIndex))))
      (CallFunction|AddGoalforIndex _array_element))
    (return)
    (else
      (bind _returnvalue (Utilities|Array|Add (Variables|Donottouch!|GetCurrentGoalIndices) (LocalVariables|GetlocalIndex)))
      (if (> _returnvalue (Utilities|Array|LastIndex (Variables|Donottouch!|GetCurrentHuntedAmounts)))
        (Utilities|Array|Add (Variables|Donottouch!|GetCurrentHuntedAmounts) 0))
      (Utilities|Array|Add (Variables|Donottouch!|GetCurrentGoals) (CallFunction|GoalatIndex (LocalVariables|GetlocalIndex)))
      (bind _returnvalue_2 (UserInterface|CreateWidget "/Game/QuestSystem/Widgets/SubGoalWidget.SubGoalWidget_C" 0 (CallFunction|GoalatIndex (LocalVariables|GetlocalIndex)) self (Variables|Donottouch!|GetQuestWidget)))
      (Utilities|Array|Add (Variables|/Game/QuestSystem/Widgets/QuestWidget.QuestWidget_C|GetSubGoalWidgets _questwidget) _returnvalue_2)
      (Widget|Panel|AddChild (Variables|/Game/QuestSystem/Widgets/QuestWidget.QuestWidget_C|GetSubGoalBox _questwidget) _returnvalue_2)
      (return))))

(fn RemoveWidgets
  (bind _questmanager (Variables|Donottouch!|GetQuestManager))
  (bind _listentrywidget (Variables|DoNotTouch!|GetListEntryWidget))
  (bind _mainwidget (Variables|/Game/QuestSystem/Blueprints/Actors/Bp_QuestManager.Bp_QuestManager_C|GetMainWidget _questmanager))
  (Utilities|Array|RemoveItem (Variables|/Game/QuestSystem/Widgets/MainWidget.MainWidget_C|GetQuestWidgets _mainwidget) (Variables|Donottouch!|GetQuestWidget))
  (Utilities|Array|RemoveItem (Variables|/Game/QuestSystem/Widgets/QuestJournal.QuestJournal_C|GetAllQuestEntries (Variables|/Game/QuestSystem/Widgets/MainWidget.MainWidget_C|GetJournal _mainwidget)) _listentrywidget)
  (Widget|RemovefromParent _listentrywidget)
  (return))