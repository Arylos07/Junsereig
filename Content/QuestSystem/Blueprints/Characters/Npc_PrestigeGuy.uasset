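; Quest-giver NPC that offers its quest once the player's prestige in a required region reaches a threshold.
; Quest-load and prestige-gain events unlock the offer and show a question mark, with loading also restoring the given state if the quest manager already holds the quest.
; Interaction starts the quest, hides the marker and swaps the dialogue, otherwise deferring to the parent.
; Cancelling the quest re-enables the offer.
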(event EventBeginPlay
  (|CallParentFunction))

(event Collision|EventActorBeginOverlap
  (params (OtherActor :type Actor%20Object%20Reference)))

(event EventOnOwnQuestCancelled
  (params (Class :type Bp%20Master%20Quest%20Class%20Reference))
  (Variables|Default|SetCanGiveQuest? true)
  (Variables|Default|SetHasGivenQuest? false)
  (Rendering|SetVisibility (Variables|Default|GetQuestionMark) true false))

(event EventTick
  (params (DeltaSeconds :type Float%20%28single-precision%29)))

(event EventOnPlayerGainPrestige
  (params (Player :type Third%20Person%20Character%20Object%20Reference))
  (bind _requiredprestige (Variables|Default|GetRequiredPrestige))
  (bind (_region _prestige) (Utilities|Struct|Breaks_RegionPrestige _requiredprestige))
  (if (Math|Boolean|ANDBoolean (>= (Default|GetPrestigebyRegion Player _region) _prestige) (not (Variables|Default|GetCanGiveQuest?)) (not (Variables|Default|GetHasGivenQuest?)))
    (Variables|Default|SetCanGiveQuest? true)
    (Rendering|SetVisibility (Variables|Default|GetQuestionMark) true false)))

(event EventOnQuestsLoaded
  (params (Manager :type Bp%20Quest%20Manager%20Object%20Reference))
  (bind _requiredprestige (Variables|Default|GetRequiredPrestige))
  (bind (_region _prestige) (Utilities|Struct|Breaks_RegionPrestige _requiredprestige))
  (if (>= (Default|GetPrestigebyRegion (Variables|/Game/QuestSystem/Blueprints/Actors/Bp_QuestManager.Bp_QuestManager_C|GetThirdPersonChar Manager) _region) _prestige)
    (Variables|Default|SetCanGiveQuest? true)
    (if (Utilities|Array|ContainsItem (Variables|/Game/QuestSystem/Blueprints/Actors/Bp_QuestManager.Bp_QuestManager_C|GetAllQuestClasses Manager) (Variables|Default|GetQuestToGive))
      (Variables|Default|SetHasGivenQuest? true)
      (Variables|Default|SetDefaultMessage (Variables|Default|GetMsgAfterQuestGiven))
      (else
        (Rendering|SetVisibility (Variables|Default|GetQuestionMark) true false)))))

(event EventOnInteractwith
  (params (Character :type Third%20Person%20Character%20Object%20Reference))
  (if (and (Variables|Default|GetCanGiveQuest?) (not (Variables|Default|GetHasGivenQuest?)))
    (Default|AddNewQuest (Variables|/Game/QuestSystem/Blueprints/Characters/ThirdPersonCharacter.ThirdPersonCharacter_C|GetQuestManagerRef Character) (Variables|Default|GetQuestToGive) true)
    (Variables|Default|SetHasGivenQuest? true)
    (Variables|Default|SetDefaultMessage (Variables|Default|GetMsgAfterQuestGiven))
    (Rendering|SetVisibility (Variables|Default|GetQuestionMark) false false)
    (else
      (|CallParentFunction Character))))

(fn ConstructionScript
  (|CallParentFunction))